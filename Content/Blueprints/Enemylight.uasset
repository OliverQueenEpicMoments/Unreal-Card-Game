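; Enemylight is a stage light actor that can be switched on and off, starting dark when play begins.
; TurnOff and Turnon events toggle the SpotLight's visibility and swap the StageLight static mesh between lit and unlit versions, rescaling it to match each mesh.
; The Blueprint only exposes these events and contains no logic that decides when the light turns on.
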(event EventBeginPlay
  (CallFunction|TurnOff))

(event Collision|EventActorBeginOverlap
  (params (OtherActor :type Actor%20Object%20Reference)))

(event EventTick
  (params (DeltaSeconds :type Float%20%28single-precision%29)))

(event EventTurnOff
  (bind _stagelight (Variables|Default|GetStageLight))
  ;[0.05098 0.05098 0.05098] Disables the light and swaps mesh accordingly
  (Rendering|SetVisibility (Variables|Default|GetSpotLight) false false)
  (Components|StaticMesh|SetStaticMesh _stagelight (Variables|Default|GetLightsOffMesh))
  (Transformation|SetWorldScale3D _stagelight "0.650000,0.650000,0.650000"))

(event EventTurnon
  (bind _stagelight (Variables|Default|GetStageLight))
  ;[0.05098 0.05098 0.05098] Enables the light and swaps mesh accordingly
  (Rendering|SetVisibility (Variables|Default|GetSpotLight) true false)
  (Components|StaticMesh|SetStaticMesh _stagelight (Variables|Default|GetLightsOnMesh))
  (Transformation|SetWorldScale3D _stagelight "1.000000,1.000000,1.000000"))

(fn ConstructionScript)