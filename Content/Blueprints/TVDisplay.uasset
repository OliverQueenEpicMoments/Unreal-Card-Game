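; TVDisplay drives an on-screen TV widget that reveals the opponent's first card in a card game.
; On BeginPlay it caches the first existing WB_TVDisplay widget and hides it.
; RevealCard finds the first actor implementing IEnemy, shows the widget and passes it that enemy's first-card message.
; ShowUI and HideUI toggle the widget's visibility, with HideUI also calling the widget's own Hide.
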(event Custom|RevealCard
  (bind _wb_display (Variables|Default|GetWB_Display))
  ;[0.05098 0.05098 0.05098] Reveals the opponents first card
  (bind _outactors (Actor|GetAllActorswithInterface "/Game/Blueprints/Interfaces/IEnemy.IEnemy_C"))
  (bind _output_get (Variables|Default|SetEnemy (Utilities|Array|Get(acopy) _outactors)))
  (Variables|/Script/UMG.Widget|SetVisibility _wb_display "Visible")
  (bind _firstcardval (Class|IEnemy|GetFirstCard(Message) _output_get))
  (Default|DisplayInitialCard _wb_display _firstcardval))

(event EventBeginPlay
  ;[0.05098 0.05098 0.05098] Setting variables and hiding self
  (bind _foundwidgets (Widget|GetAllWidgetsOfClass "/Game/UI/WB_TVDisplay.WB_TVDisplay_C" false))
  (bind _output_get (Variables|Default|SetWB_Display (Utilities|Array|Get(acopy) _foundwidgets)))
  (Variables|/Script/UMG.Widget|SetVisibility _output_get "Hidden"))

(event Collision|EventActorBeginOverlap
  (params (OtherActor :type Actor%20Object%20Reference)))

(event EventTick
  (params (DeltaSeconds :type Float%20%28single-precision%29)))

(event EventShowUI
  ;[0.05098 0.05098 0.05098] Shows the widget
  (Variables|/Script/UMG.Widget|SetVisibility (Variables|Default|GetWB_Display) "Visible"))

(event EventHideUI
  (bind _wb_display (Variables|Default|GetWB_Display))
  ;[0.05098 0.05098 0.05098] Hides the widget
  (Variables|/Script/UMG.Widget|SetVisibility _wb_display "Hidden")
  (Default|Hide _wb_display))

(fn ConstructionScript)