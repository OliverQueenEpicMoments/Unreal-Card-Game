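; OverheadLight is an overhead light fixture Blueprint that can be switched on and off.
; TurnOff and Turnon events toggle the SpotLight's visibility and swap the first material slot on the OverheadLight component between lit and unlit materials to match.
; It has no active BeginPlay, overlap, Tick or construction logic, so switching only happens when those events are called.
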(event EventBeginPlay)

(event Collision|EventActorBeginOverlap
  (params (OtherActor :type Actor%20Object%20Reference)))

(event EventTick
  (params (DeltaSeconds :type Float%20%28single-precision%29)))

(event EventTurnOff
  ;[0.05098 0.05098 0.05098] Disables the light and swaps the material accordingly
  (Rendering|SetVisibility (Variables|Default|GetSpotLight) false false)
  (Rendering|Material|SetMaterial (Variables|Default|GetOverheadLight) 0 (Variables|Default|GetLightsOffMaterial)))

(event EventTurnon
  ;[0.05098 0.05098 0.05098] Enables the light and swaps the material accordingly
  (Rendering|SetVisibility (Variables|Default|GetSpotLight) true false)
  (Rendering|Material|SetMaterial (Variables|Default|GetOverheadLight) 0 (Variables|Default|GetLightsOnMaterial)))

(fn ConstructionScript)