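; TVDisplays is an actor Blueprint that drives the in-game TV display widget, showing card results and random creepy messages.
; On BeginPlay it caches the first WB_TVDisplays widget found and plays one of three messages: DeadSpace, Robot or HelpMe.
; ShowWinner forwards both players' card values to that widget.
; ShowUI and HideUI toggle its visibility, with ShowUI also picking a new random message.
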(event Custom|ShowWinner
  (params (PlayerCardVal :type Integer) (EnemyCardVal :type Integer))
  ;[0.05098 0.05098 0.05098] Displays the card values of both players
  (Default|ShowWinner (Variables|Default|GetWB_Displays) PlayerCardVal EnemyCardVal))

(event Custom|CreepyMessages
  (bind _wb_displays (Variables|Default|GetWB_Displays))
  ;[0.05098 0.05098 0.05098] Displays a creepy message at random
  (switch int (Math|Random|RandomIntegerinRange 0 2)
    (:0
      (Default|DeadSpace _wb_displays))
    (:1
      (Default|Robot _wb_displays))
    (:2
      (Default|HelpMe _wb_displays))))

(event EventBeginPlay
  ;[0.05098 0.05098 0.05098] Setting variables
  (bind _foundwidgets (Widget|GetAllWidgetsOfClass "/Game/UI/WB_TVDisplays.WB_TVDisplays_C" false))
  (Variables|Default|SetWB_Displays (Utilities|Array|Get(acopy) _foundwidgets))
  (CallFunction|CreepyMessages))

(event Collision|EventActorBeginOverlap
  (params (OtherActor :type Actor%20Object%20Reference)))

(event EventTick
  (params (DeltaSeconds :type Float%20%28single-precision%29)))

(event EventShowUI
  ;[0.05098 0.05098 0.05098] Shows the widget
  (Variables|/Script/UMG.Widget|SetVisibility (Variables|Default|GetWB_Displays) "Visible")
  (CallFunction|CreepyMessages))

(event EventHideUI
  ;[0.05098 0.05098 0.05098] Hides the widget
  (Variables|/Script/UMG.Widget|SetVisibility (Variables|Default|GetWB_Displays) "Hidden"))

(fn ConstructionScript)