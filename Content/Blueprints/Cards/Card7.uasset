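; Card7 is a playing card actor worth 7, shown on a plane mesh and owned by either the player or the enemy.
; The construction script sets its value and picks the face-up or face-down material, and ReturnCardValue exposes that value.
; Events flip it face down, tag it by owner, or burn it by swapping to a dissolve material and destroying it after a short delay.
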(event EventBeginPlay)

(event Collision|EventActorBeginOverlap
  (params (OtherActor :type Actor%20Object%20Reference)))

(event EventTick
  (params (DeltaSeconds :type Float%20%28single-precision%29)))

(event EventSetCardOwner
  (params (IsPlayers :type Boolean))
  ;[0.05098 0.05098 0.05098] Assigns tag based on which player this card belongs to
  (if IsPlayers
    (bind _output_get (Variables|Default|SetBelongsTo "Player"))
    (Variables|Default|SetTags (Utilities|Array|MakeArray _output_get))
    (else
      (bind _output_get_2 (Variables|Default|SetBelongsTo "Enemy"))
      (Variables|Default|SetTags (Utilities|Array|MakeArray _output_get_2)))))

(event EventFaceDown
  ;[0.05098 0.05098 0.05098] Hides this cards value by making it face down
  (Rendering|Material|SetMaterial (Variables|Default|GetPlane) 0 "/Game/Materials/Cards/CardFaceDown.CardFaceDown"))

(event EventBurn
  ;[0.05098 0.05098 0.05098] Starts burning effect and destroys self
  (Rendering|Material|SetMaterial (Variables|Default|GetPlane) 0 "/Game/Materials/Effects/CardDissolve.CardDissolve")
  (Utilities|FlowControl|Delay 1.0)
  (Actor|DestroyActor))

(fn ConstructionScript
  (bind _plane (Variables|Default|GetPlane))
  (Variables|Default|SetValue 7)
  (if (Variables|Default|GetIsFaceDown)
    (Rendering|Material|SetMaterial _plane 0 "/Game/Materials/Cards/CardFaceDown.CardFaceDown")
    (else
      (Rendering|Material|SetMaterial _plane 0 "/Game/Materials/Cards/Card7Material.Card7Material"))))

(fn ReturnCardValue
  (return (Variables|Default|GetValue)))