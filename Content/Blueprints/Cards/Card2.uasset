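; Card2 is a card actor Blueprint representing a card with a value of 2, shown on a plane mesh.
; Its construction script sets the value and picks the face-down or Card2 face material from the IsFaceDown flag.
; Events flip it to the face-down material and tag it as Player or Enemy owned through gameplay tags.
; The Burn event and Tick are empty.
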(event EventBeginPlay)

(event Collision|EventActorBeginOverlap
  (params (OtherActor :type Actor%20Object%20Reference)))

(event EventTick
  (params (DeltaSeconds :type Float%20%28single-precision%29)))

(event EventBurn)

(event EventFaceDown
  (Rendering|Material|SetMaterial (Variables|Default|GetPlane) 0 "/Game/Materials/Cards/CardFaceDown.CardFaceDown"))

(event EventSetCardOwner
  (params (IsPlayers :type Boolean))
  (bind _gameplaytags (Variables|Default|GetGameplayTags))
  (if IsPlayers
    (GameplayTags|AddGameplayTag _gameplaytags "(TagName=\"Player\")" :!class /Script/GameplayTags.BlueprintGameplayTagLibrary)
    (else
      (GameplayTags|AddGameplayTag _gameplaytags "(TagName=\"Enemy\")" :!class /Script/GameplayTags.BlueprintGameplayTagLibrary))))

(fn ConstructionScript
  (bind _plane (Variables|Default|GetPlane))
  (Variables|Default|SetValue 2)
  (if (Variables|Default|GetIsFaceDown)
    (Rendering|Material|SetMaterial _plane 0 "/Game/Materials/Cards/CardFaceDown.CardFaceDown")
    (else
      (Rendering|Material|SetMaterial _plane 0 "/Game/Materials/Cards/Card2Material.Card2Material"))))