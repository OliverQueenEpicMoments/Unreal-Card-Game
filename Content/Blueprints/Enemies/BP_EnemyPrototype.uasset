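; Prototype enemy opponent for a turn-based card game, driven by turn events from BP_FirstPersonGameMode.
; On BeginPlay it binds Play to the game mode's enemy-turn event.
; While IsMyTurn reports the enemy's turn, Play draws cards through the Table actor, calls SwitchTurn and rechecks, then prints that the turn is over.
; It makes no card choices, and ReturnCardValue is a stub returning zero.
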(event Custom|Play
  (bind _ismyturn (CallFunction|IsMyTurn))
  (bind _output_get (Variables|Default|SetMyTurn _ismyturn))
  (while _output_get
    (bind _returnvalue (Actor|GetActorOfClass "/Game/Blueprints/Table.Table_C"))
    (Default|DrawCards _returnvalue false)
    (bind _returnvalue_2 (Actor|GetActorOfClass "/Game/FirstPerson/Blueprints/BP_FirstPersonGameMode.BP_FirstPersonGameMode_C"))
    (Default|SwitchTurn _returnvalue_2)
    (bind _ismyturn_2 (CallFunction|IsMyTurn))
    (Variables|Default|SetMyTurn _ismyturn_2))
  (Development|PrintString "Enemy turn over"))

(event EventBeginPlay
  (bind _returnvalue (Actor|GetActorOfClass "/Game/FirstPerson/Blueprints/BP_FirstPersonGameMode.BP_FirstPersonGameMode_C"))
  (EventDispatchers|BindEventtoOnEnemyTurn _returnvalue (delegate Custom|Play)))

(event Collision|EventActorBeginOverlap
  (params (OtherActor :type Actor%20Object%20Reference)))

(event EventTick
  (params (DeltaSeconds :type Float%20%28single-precision%29)))

(fn ConstructionScript)

(fn IsMyTurn
  (bind _returnvalue (Actor|GetActorOfClass "/Game/FirstPerson/Blueprints/BP_FirstPersonGameMode.BP_FirstPersonGameMode_C"))
  (bind _turn (Default|GetCurrentTurn _returnvalue))
  (return (Utilities|Enum|Equal(Enum) _turn "NewEnumerator1")))

(fn ReturnCardValue
  (return 0))