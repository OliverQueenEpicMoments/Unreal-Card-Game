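; BP_SoldierEnemy is the AI opponent in a turn-based card game, with health, healing and death that requests a replacement enemy from the level.
; It mirrors its turn state into the AI blackboard each Tick and exposes draw and pass actions that drive table, animation and game mode.
; Card totals come from "Enemy"-tagged actors; the UI omits the first card's value, which is added back afterwards.
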(event Custom|Play
  ;[0.05098 0.05098 0.05098] Main loop for when it's this players turn
  (bind _ismyturn (CallFunction|IsMyTurn))
  (Variables|Default|SetMyTurn _ismyturn))

(event Custom|Death
  ;[0.05098 0.05098 0.05098] Self-explanatory
  (Variables|Default|SetIsDead true)
  (Default|CallOnDeath)
  (Utilities|FlowControl|Delay 7.0)
  (Actor|DestroyActor)
  (Class|IGameData|GetNewEnemy(Message) (Variables|Default|GetLevelBP)))

(event Custom|ResetRound
  ;[0.05098 0.05098 0.05098] Resets UI at the start of a new round
  (Default|InitializeUI (Variables|Default|GetWB_EnemyUI) (Variables|Default|GetGoal)))

(event EventBeginPlay
  ;[0.05098 0.05098 0.05098] Initializing UI and events
  (bind _foundwidgets (Widget|GetAllWidgetsOfClass "/Game/UI/WB_EnemyCardDisplay.WB_EnemyCardDisplay_C" false))
  (bind _output_get (Variables|Default|SetWB_EnemyUI (Utilities|Array|Get(acopy) _foundwidgets)))
  (Default|InitializeUI _output_get (Variables|Default|GetGoal))
  (bind _returnvalue (Actor|GetActorOfClass "/Game/FirstPerson/Blueprints/BP_FirstPersonGameMode.BP_FirstPersonGameMode_C"))
  (bind _output_get_2 (Variables|Default|SetGameModeBP _returnvalue))
  (EventDispatchers|BindEventtoOnEnemyTurn _output_get_2 (delegate Custom|Play))
  (bind _returnvalue_2 (Actor|GetActorOfClass "/Game/Blueprints/Table.Table_C"))
  (EventDispatchers|BindEventtoOnPlayerReset _returnvalue_2 (delegate Custom|ResetRound))
  (Variables|Default|SetAnimBP (Components|SkeletalMesh|GetAnimInstance (Variables|Character|GetMesh)))
  (bind _returnvalue_3 (Actor|GetActorOfClass "/Game/Blueprints/BetterLevelBP.BetterLevelBP_C"))
  (Variables|Default|SetLevelBP _returnvalue_3)
  (bind _returnvalue_4 (Actor|GetActorOfClass "/Game/Blueprints/Table.Table_C"))
  (Variables|Default|SetTableBP _returnvalue_4))

(event Collision|EventActorBeginOverlap
  (params (OtherActor :type Actor%20Object%20Reference)))

(event EventPassTurn
  ;[0.05098 0.05098 0.05098] Passes this turn
  (bind _ismyturn (CallFunction|IsMyTurn))
  (if _ismyturn
    (Class|IAnimated|PassTurnAnimation(Message) (Variables|Default|GetAnimBP))
    (Class|IGameData|EnemyPassState(Message) (Variables|Default|GetGameModeBP) true)
    (Default|SwitchTurn2 (Variables|Default|GetGameModeBP))))

(event EventTick
  (params (DeltaSeconds :type Float%20%28single-precision%29))
  (bind _returnvalue (Utilities|Name|MakeLiteralName "IsTurn"))
  (bind _self self)
  (bind _myturn (Variables|Default|GetMyTurn))
  (bind _returnvalue_2 (AI|GetAIController _self))
  (bind _returnvalue_3 (AI|GetBlackboard _returnvalue_2))
  ;[0.05098 0.05098 0.05098] Setting blackboard values
  (if _myturn
    (AI|Components|Blackboard|SetValueasBool _returnvalue_3 _returnvalue _myturn)
    (else
      (AI|Components|Blackboard|SetValueasBool _returnvalue_3 _returnvalue _myturn))))

(event Game|Damage|EventAnyDamage
  (params (Damage :type Float%20%28single-precision%29) (DamageType :type Damage%20Type%20Object%20Reference) (InstigatedBy :type Controller%20Object%20Reference) (DamageCauser :type Actor%20Object%20Reference))
  ;[0.05098 0.05098 0.05098] Taking damage
  (if (not (Variables|Default|GetIsDead))
    (Variables|Default|SetCurrentHealth (Math|Float|Clamp(Float) (- (Variables|Default|GetCurrentHealth) Damage) 0.0 (Variables|Default|GetMaxHealth)))
    (if (<= (Variables|Default|GetCurrentHealth) 0.0)
      (CallFunction|Death)
      (else
        (Default|CallOnHurt)))))

(event EventHealPlayer
  (params (HealValue :type Float%20%28double-precision%29))
  ;[0.05098 0.05098 0.05098] For healing this player
  (if (not (Variables|Default|GetIsDead))
    (Variables|Default|SetCurrentHealth (Math|Float|Clamp(Float) (+ (Variables|Default|GetCurrentHealth) HealValue) 0.0 (Variables|Default|GetMaxHealth)))))

(event EventResetScore
  ;[0.05098 0.05098 0.05098] Resets this players card values
  (Variables|Default|SetCardValue 0)
  (Variables|Default|SetFirstCard 0))

(event EventUpdateCardValues
  (params (IsPlayers :type Boolean))
  ;[0.05098 0.05098 0.05098] Updates the enemies current card values
  (Variables|Default|SetCardValue 0)
  (if (not IsPlayers)
    (bind _outactors (Actor|GetAllActorswithTag "Enemy"))
    (for (_array_element _array_index) _outactors
      (if (== 0 _array_index)
        (bind _cardvalue (Class|ICards|ReturnCardValue(Message) _array_element))
        (Variables|Default|SetFirstCard _cardvalue)
        (else
          (bind _cardvalue_2 (Class|ICards|ReturnCardValue(Message) _array_element))
          (Variables|Default|SetCardValue (+ _cardvalue_2 (Variables|Default|GetCardValue))))))
    (Default|UpdateCardUI (Variables|Default|GetWB_EnemyUI) (Variables|Default|GetCardValue) (Variables|Default|GetGoal))
    (Variables|Default|SetCardValue (+ (Variables|Default|GetFirstCard) (Variables|Default|GetCardValue)))))

(fn ConstructionScript
  (Variables|Default|SetCurrentHealth (Variables|Default|GetMaxHealth)))

(fn DrawCard
  (bind _gamemodebp (Variables|Default|GetGameModeBP))
  (bind _ismyturn (CallFunction|IsMyTurn))
  (if _ismyturn
    (Default|DrawCards (Variables|Default|GetTableBP) false)
    (Class|IAnimated|DrawCardAnimation(Message) (Variables|Default|GetAnimBP))
    (Class|IGameData|EnemyPassState(Message) _gamemodebp false)
    (Default|SwitchTurn2 _gamemodebp)
    (return true)
    (else
      (return false))))

(fn IsMyTurn
  (bind _turn (Default|GetCurrentTurn (Variables|Default|GetGameModeBP)))
  (return (Utilities|Enum|Equal(Enum) _turn "NewEnumerator1")))

(fn ReturnCardValue
  (return (Variables|Default|GetCardValue)))

(fn ReturnFalseCardValue
  (return 0))