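; BP_Zombie is a zombie enemy, filed among the easy enemies, that handles taking damage and dying.
; AnyDamage subtracts from clamped health while it is alive, then fires either the OnHurt dispatcher or, at zero health, the Death event.
; Death sets IsDead, fires OnDeath, destroys the actor after a delay and calls GetNewEnemyMessage on the level Blueprint reference.
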(event Custom|Death
  ;[0.05098 0.05098 0.05098] Self-explanatory
  (Variables|Default|SetIsDead true)
  (Default|CallOnDeath)
  (Utilities|FlowControl|Delay 7.0)
  (Actor|DestroyActor)
  (Class|IGameData|GetNewEnemy(Message) (Variables|Default|GetLevelBP)))

(event EventBeginPlay
  (|CallParentFunction) ; This node is disabled and will not be called.\nDrag off pins to build functionality.
)

(event Collision|EventActorBeginOverlap
  (params (OtherActor :type Actor%20Object%20Reference)))

(event EventTick
  (params (DeltaSeconds :type Float%20%28single-precision%29))
  (|CallParentFunction DeltaSeconds) ; This node is disabled and will not be called.\nDrag off pins to build functionality.
)

(event Game|Damage|EventAnyDamage
  (params (Damage :type Float%20%28single-precision%29) (DamageType :type Damage%20Type%20Object%20Reference) (InstigatedBy :type Controller%20Object%20Reference) (DamageCauser :type Actor%20Object%20Reference))
  ;[0.05098 0.05098 0.05098] Taking damage
  (if (not (Variables|Default|GetIsDead))
    (Variables|Default|SetCurrentHealth (Math|Float|Clamp(Float) (- (Variables|Default|GetCurrentHealth) Damage) 0.0 (Variables|Default|GetMaxHealth)))
    (if (<= (Variables|Default|GetCurrentHealth) 0.0)
      (CallFunction|Death)
      (else
        (Default|CallOnHurt)))))

(fn ConstructionScript
  (|CallParentFunction))