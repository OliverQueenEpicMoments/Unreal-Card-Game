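; The Empress tarot card, which changes the card game's goal from 21 to 27 when it spawns.
; On BeginPlay it runs the parent logic, finds BP_FirstPersonGameMode with GetActorOfClass and passes NewGoal to its ChangeGoalMessage.
; It then calls FadeAway, with no overlap or tick logic of its own.
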(event EventBeginPlay
  ;[0.05098 0.05098 0.05098] Sets the card goal to 27 instead of 21
  (|CallParentFunction)
  (bind _returnvalue (Actor|GetActorOfClass "/Game/FirstPerson/Blueprints/BP_FirstPersonGameMode.BP_FirstPersonGameMode_C"))
  (bind _output_get (Variables|Default|SetGameModeBP _returnvalue))
  (Class|IGameData|ChangeGoal(Message) _output_get (Variables|Default|GetNew%20Goal))
  (CallFunction|FadeAway))

(event Collision|EventActorBeginOverlap
  (params (OtherActor :type Actor%20Object%20Reference))
  (|CallParentFunction OtherActor) ; This node is disabled and will not be called.\nDrag off pins to build functionality.
)

(event EventTick
  (params (DeltaSeconds :type Float%20%28single-precision%29))
  (|CallParentFunction DeltaSeconds) ; This node is disabled and will not be called.\nDrag off pins to build functionality.
)

(fn ConstructionScript
  (|CallParentFunction))