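; The Moon tarot card actor, which destroys the most recently drawn card as its effect.
; On BeginPlay it runs the parent logic, calls UndoCard on the BP_FirstPersonGameMode actor and starts FadeAway.
; After a short delay it tells that game mode to update the player UI.
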(event EventBeginPlay
  ;[0.05098 0.05098 0.05098] Destroys the most recently drawn card
  (|CallParentFunction)
  (bind _returnvalue (Actor|GetActorOfClass "/Game/FirstPerson/Blueprints/BP_FirstPersonGameMode.BP_FirstPersonGameMode_C"))
  (Default|UndoCard _returnvalue)
  (CallFunction|FadeAway)
  (Utilities|FlowControl|Delay 3.0)
  (Default|UpdatePlayerUI _returnvalue))

(event Collision|EventActorBeginOverlap
  (params (OtherActor :type Actor%20Object%20Reference))
  (|CallParentFunction OtherActor) ; This node is disabled and will not be called.\nDrag off pins to build functionality.
)

(event EventTick
  (params (DeltaSeconds :type Float%20%28single-precision%29))
  (|CallParentFunction DeltaSeconds) ; This node is disabled and will not be called.\nDrag off pins to build functionality.
)

(fn ConstructionScript
  (|CallParentFunction))