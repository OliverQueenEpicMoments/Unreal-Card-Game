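; Base actor for a tarot card that announces its name and description on screen, with support for fading away.
; The construction script applies the card's material to its plane.
; On BeginPlay it finds the first existing WB_TarotInfo widget, makes it visible and passes it the card's text.
; FadeAway waits, swaps the plane to a dissolve material, then destroys the actor after another delay.
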(event EventBeginPlay
  ;[0.05098 0.05098 0.05098] Initializing UI pop up
  (bind _foundwidgets (Widget|GetAllWidgetsOfClass "/Game/UI/WB_TarotInfo.WB_TarotInfo_C" false))
  (Variables|/Script/UMG.Widget|SetVisibility (Utilities|Array|Get(acopy) _foundwidgets) "Visible")
  (Default|UpdatePopUp (Utilities|Array|Get(acopy) _foundwidgets) (Variables|Default|GetName) (Variables|Default|GetDescription)))

(event Collision|EventActorBeginOverlap
  (params (OtherActor :type Actor%20Object%20Reference)))

(event EventTick
  (params (DeltaSeconds :type Float%20%28single-precision%29)))

(event EventFadeAway
  ;[0.05098 0.05098 0.05098] Fades the card away after displaying its name and what it does
  (Utilities|FlowControl|Delay 3.0)
  (Rendering|Material|SetMaterial (Variables|Default|GetPlane) 0 "/Game/Materials/Effects/CardDissolve.CardDissolve")
  (Utilities|FlowControl|Delay 2.0)
  (Actor|DestroyActor))

(fn ConstructionScript
  (Rendering|Material|SetMaterial (Variables|Default|GetPlane) 0 (Variables|Default|GetCardMaterial)))