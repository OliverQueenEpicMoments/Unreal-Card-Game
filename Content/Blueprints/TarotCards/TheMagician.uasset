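; The Magician tarot card Blueprint, an enemy-only card that makes the enemy disappear when drawn.
; On BeginPlay it runs the parent logic, finds actors implementing the IEnemy interface and sends MagicianDisappearMessage to the first one.
; It then plays the GetOutLoud sound and calls FadeAway to fade the card.
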(event EventBeginPlay
  ;[0.05098 0.05098 0.05098] Disappears the enemy when drawn (enemy only tarot)
  (|CallParentFunction)
  (bind _outactors (Actor|GetAllActorswithInterface "/Game/Blueprints/Interfaces/IEnemy.IEnemy_C"))
  (Class|IEnemy|MagicianDisappear(Message) (Utilities|Array|Get(acopy) _outactors))
  (Audio|PlaySound2D "/Game/Sounds/GetOutLoud.GetOutLoud" 1.0 1.0 0.0 0 0)
  (CallFunction|FadeAway))

(event Collision|EventActorBeginOverlap
  (params (OtherActor :type Actor%20Object%20Reference))
  (|CallParentFunction OtherActor) ; This node is disabled and will not be called.\nDrag off pins to build functionality.
)

(event EventTick
  (params (DeltaSeconds :type Float%20%28single-precision%29))
  (|CallParentFunction DeltaSeconds) ; This node is disabled and will not be called.\nDrag off pins to build functionality.
)

(fn ConstructionScript
  (|CallParentFunction))