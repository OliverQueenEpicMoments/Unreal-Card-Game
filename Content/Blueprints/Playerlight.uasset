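; Playerlight is a stage spotlight actor that can be switched on, switched off, or turned off for a timed interval.
; TurnOff and Turnon toggle the SpotLight's visibility and swap the StageLight mesh and scale to match.
; Turning on also plays a spotlight sound, positioned using the mesh's relative location rather than its world location.
; TurnOffThenon chains both events around a Delay of caller-supplied length.
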(event EventBeginPlay)

(event Collision|EventActorBeginOverlap
  (params (OtherActor :type Actor%20Object%20Reference)))

(event EventTick
  (params (DeltaSeconds :type Float%20%28single-precision%29)))

(event EventTurnOffThenon
  (params (OffLength :type Float%20%28double-precision%29))
  ;[0.05098 0.05098 0.05098] Turns off the light, then after the specified time turns it back on
  (CallFunction|TurnOff)
  (Utilities|FlowControl|Delay OffLength)
  (CallFunction|Turnon))

(event EventTurnOff
  (bind _stagelight (Variables|Default|GetStageLight))
  ;[0.05098 0.05098 0.05098] Disables the light and swaps mesh accordingly
  (Rendering|SetVisibility (Variables|Default|GetSpotLight) false false)
  (Components|StaticMesh|SetStaticMesh _stagelight (Variables|Default|GetLightsOffMesh))
  (Transformation|SetWorldScale3D _stagelight "0.650000,0.650000,0.650000"))

(event EventTurnon
  (bind _stagelight (Variables|Default|GetStageLight))
  ;[0.05098 0.05098 0.05098] Enables the light and swaps mesh accordingly
  (Rendering|SetVisibility (Variables|Default|GetSpotLight) true false)
  (Components|StaticMesh|SetStaticMesh _stagelight (Variables|Default|GetLightsOnMesh))
  (Transformation|SetWorldScale3D _stagelight "1.000000,1.000000,1.000000")
  (Audio|PlaySoundatLocation "/Game/Sounds/SpotlightOn.SpotlightOn" (Variables|/Script/Engine.SceneComponent|GetRelativeLocation (Variables|Default|GetStageLight)) "0, 0, 0" 1.0 1.0 0.0 0 0 0 0))

(fn ConstructionScript)